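; Zombie AI controller that sends its pawn walking to a random waypoint when play begins.
; BeginPlay caches every TargetPoint in the level as Waypoints, then issues a single SimpleMoveToActor to a randomly picked one, with no repeat on arrival.
; GoToPlayer is an unfinished stub: it calls MoveToActor with no goal and is not called in this graph.
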(event `self.ReceiveBeginPlay`
  (`|ExecutionSequence`
    (:`then_0`
      (bind _outactors (`GameplayStatics.GetAllActorsOfClass` "/Script/Engine.TargetPoint"))
      (set `self.Waypoints` _outactors))
    (:`then_1`
      (`self.Go to random waypoint`))))

(fn `Get random waypoint`
  (returns (NewParam :type "TargetPoint Object Reference"))
  (bind _waypoints (`self.Waypoints`))
  (return (`|GetArrayItem` _waypoints (`KismetMathLibrary.RandomIntegerInRange` 0 (- (`KismetArrayLibrary.Array_Length` _waypoints) 1)))))

(fn `Go to player`
  (`self.MoveToActor` null -1.0 true true true null))

(fn `Go to random waypoint`
  (`AIBlueprintHelperLibrary.SimpleMoveToActor` self (`self.Get random waypoint`)))

(fn `UserConstructionScript`)