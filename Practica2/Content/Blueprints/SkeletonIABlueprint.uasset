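; AI controller for a skeleton that sends it walking to a randomly chosen TargetPoint in the level.
; On both BeginPlay and Possess it gathers every TargetPoint into Waypoints, then issues a SimpleMoveToActor to a random entry.
; Nothing picks another waypoint on arrival, so movement is only triggered by those two events.
; GoToPlayer is an unfinished stub: its MoveToActor has no goal and nothing in the file calls it.
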(event `self.ReceiveBeginPlay`
  ;[1 1 1] Obtiene los waypoint al iniciar
  (`|ExecutionSequence`
    (:`then_0`
      (bind _outactors (`GameplayStatics.GetAllActorsOfClass` "/Script/Engine.TargetPoint"))
      (set `self.Waypoints` _outactors))
    (:`then_1`
      (`self.Go To Random Waypoint`))))

(event `self.ReceivePossess`
  (params (PossessedPawn :type "Pawn Object Reference"))
  ;[1 1 1] Obtiene los waypoint al spawnear
  (`|ExecutionSequence`
    (:`then_0`
      (bind _outactors (`GameplayStatics.GetAllActorsOfClass` "/Script/Engine.TargetPoint"))
      (set `self.Waypoints` _outactors))
    (:`then_1`
      (`self.Go To Random Waypoint`))))

(fn `Get random waypoint`
  (returns (NewParam :type "TargetPoint Object Reference"))
  (bind _waypoints (`self.Waypoints`))
  (return (`|GetArrayItem` _waypoints (`KismetMathLibrary.RandomIntegerInRange` 0 (- (`KismetArrayLibrary.Array_Length` _waypoints) 1)))))

(fn `Go to player`
  (`self.MoveToActor` null -1.0 true true true null))

(fn `Go to random waypoint`
  (`AIBlueprintHelperLibrary.SimpleMoveToActor` self (`self.Get random waypoint`)))

(fn `UserConstructionScript`)